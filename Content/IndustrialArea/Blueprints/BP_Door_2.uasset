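; BP_Door_2 is a key-locked door in the IndustrialArea content that swings open when the player interacts while holding a key.
; BeginPlay caches the player as a VisceraCharacter, and Interact checks that character's HasKey flag before calling Open.
; Open plays a timeline that drives the relative yaw of the SMDoor2 component, with no closing logic or locked-door feedback.
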(event Custom|Open
  (bind _tet (Timeline|Timeline_0 Play)
    (:Update
      (Transformation|SetRelativeRotation (Variables|Default|GetSM_Door_2) (Math|Rotator|MakeRotator 0.0 0.0 _tet) false false))))

(event EventBeginPlay
  (bind _asviscera_character (Utilities|Casting|CastToVisceraCharacter (Game|GetPlayerCharacter 0)))
  (Variables|Default|SetAs%20Viscera%20Character_0 _asviscera_character))

(event Collision|EventActorBeginOverlap
  (params (OtherActor :type Actor%20Object%20Reference)))

(event EventTick
  (params (DeltaSeconds :type Float%20%28single-precision%29)))

(event EventInteract
  (if (Variables|/Game/ThirdPersonBP/Blueprints/VisceraCharacter.VisceraCharacter_C|GetHasKey (Variables|Default|GetAs%20Viscera%20Character_0))
    (CallFunction|Open)))

(fn ConstructionScript)